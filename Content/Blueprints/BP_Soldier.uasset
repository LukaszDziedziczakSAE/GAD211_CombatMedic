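; BP_Soldier is a soldier character with modular military gear that fires an assault rifle at an opponent.
; FireWeapon uses the Combat component to fire on a living target, or acquires one if none is valid.
; Each shot faces the opponent, triggers muzzle flash and positional sound, and plays a standing or crouched montage based on Crouching.
; The construction script makes all outfit meshes follow the main Mesh's pose through leader-pose linking.
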(event `self.FireWeapon`
  (bind _combat (`self.Combat`))
  (bind _ns_ar_muzzleflash_2_once (`self.NS_AR_Muzzleflash_2_ONCE`))
  (bind _combat_2 (`self.Combat`))
  (`SoldierCombat.Opponent` _combat
    (:`then`
      (if (not (`SoldierCombat.OpponentIsDown` (`self.Combat`)))
        (`SoldierCombat.LookAtOpponent` _combat_2 :!label _label)
        (`SoldierCombat.Fire` _combat_2)
        (`ActorComponent.Activate` _ns_ar_muzzleflash_2_once true)
        (`GameplayStatics.PlaySoundAtLocation` "/Game/SFX/Gun/Cue_ARFire.Cue_ARFire" (`SceneComponent.K2_GetComponentLocation` _ns_ar_muzzleflash_2_once) (struct) 1.0 1.0 0.0 "/Game/SFX/SoundAttenuation.SoundAttenuation" null null null)
        (if (< (`self.Crouching`) 0.5)
          (`|PlayMontage` (`self.Mesh`) "/Game/Rifle_01/Animation/In-Place/WeaponFire.WeaponFire")
          (else
            (`|PlayMontage` (`self.Mesh`) "/Game/Rifle_01/Animation/In-Place/CrouchedWeaponFire.CrouchedWeaponFire")))))
    (:`else`
      (bind _returnvalue (`SoldierCombat.TrySetOpponent` _combat))
      (if _returnvalue
        (goto _label)))))

(fn `UserConstructionScript`
  (`SkinnedMeshComponent.SetLeaderPoseComponent` (`self.SK_Military_Helmet2`) (`self.Mesh`) false false)
  (`SkinnedMeshComponent.SetLeaderPoseComponent` (`self.SK_Military_Kneepad_L`) (`self.Mesh`) false false)
  (`SkinnedMeshComponent.SetLeaderPoseComponent` (`self.SK_Military_Kneepad_R`) (`self.Mesh`) false false)
  (`SkinnedMeshComponent.SetLeaderPoseComponent` (`self.SK_Military_Outfit2`) (`self.Mesh`) false false)
  (`SkinnedMeshComponent.SetLeaderPoseComponent` (`self.SK_Military_Vest1_Belt`) (`self.Mesh`) false false)
  (`SkinnedMeshComponent.SetLeaderPoseComponent` (`self.SK_Military_Headset2`) (`self.Mesh`) false false)
  (`SkinnedMeshComponent.SetLeaderPoseComponent` (`self.SK_Military_Vest1`) (`self.Mesh`) false false)
  (`SkinnedMeshComponent.SetLeaderPoseComponent` (`self.SK_Military_Helmet1_fastering`) (`self.Mesh`) false false)
  (`SkinnedMeshComponent.SetLeaderPoseComponent` (`self.SK_Military_Goggles1`) (`self.Mesh`) false false)
  (`SkinnedMeshComponent.SetLeaderPoseComponent` (`self.SK_Military_Boots4`) (`self.Mesh`) false false)
  (`SkinnedMeshComponent.SetLeaderPoseComponent` (`self.SK_Military_Pants4`) (`self.Mesh`) false false)
  (`SkinnedMeshComponent.SetLeaderPoseComponent` (`self.SK_Military_Shirt6`) (`self.Mesh`) false false)
  (`SkinnedMeshComponent.SetLeaderPoseComponent` (`self.SK_Military_Palm_Hands_Male`) (`self.Mesh`) false false))
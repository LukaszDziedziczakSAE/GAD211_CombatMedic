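; AI controller for soldier pawns that runs the soldier behavior tree and feeds its blackboard.
; On possession it caches the BP_Soldier, starts BT_Soldier and sets the Waypoint key to the soldier's first fighting position, if one is valid.
; Each tick it copies the soldier's downed state into the Downed key.
; SetWaypoint writes a given location to the Waypoint key.
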(event `self.ReceiveBeginPlay`)

(event `self.ReceivePossess`
  (params (PossessedPawn :type "Pawn Object Reference"))
  (bind _asbp_soldier (cast `/Game/Blueprints/BP_Soldier` PossessedPawn))
  (bind _output_get (set `self.Soldier` _asbp_soldier))
  (`self.RunBehaviorTree` "/Game/AI/BT_Soldier.BT_Soldier")
  (bind _fightingposition1 (`Soldier.FightingPosition1` _output_get)
    (:`then`
      (`self.Set Waypoint` (`self.K2_GetActorLocation` _fightingposition1)))
    (:`else`)))

(event `self.ReceiveTick`
  (params (DeltaSeconds :type "Float (single-precision)"))
  (bind _soldier (`self.Soldier`)
    (:`then`
      (`BlackboardComponent.SetValueAsBool` (`AIBlueprintHelperLibrary.GetBlackboard` null) "Downed" (`Soldier.IsDowned` _soldier)))
    (:`else`)))

(fn `Set Waypoint`
  (params (`Waypoint Location` :type "Vector Structure"))
  (`self.Soldier`
    (:`then`
      (bind _blackboard (`self.Blackboard`)
        (:`then`
          (`BlackboardComponent.SetValueAsVector` _blackboard "Waypoint" `Waypoint Location`))
        (:`else`)))
    (:`else`)))

(fn `UserConstructionScript`)